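; Horse actor that glides between locations by interpolating its position every Tick, without sweeping for collision.
; While ShouldMove is set, it eases toward GetMoveTargetLocation, then clears the flag and calls the horse-arrived event once within one unit.
; Otherwise it eases slightly faster toward TargetLocation, which SetTargetLocation updates.
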(event `self.ReceiveBeginPlay`)

(event `self.ReceiveTick`
  (params (DeltaSeconds :type "Float (single-precision)"))
  (bind _returnvalue (`self.K2_GetActorLocation`))
  (if (`self.ShouldMove`)
    (bind _returnvalue_2 (`self.GetMoveTargetLocation`))
    (`self.K2_SetActorLocation` (`KismetMathLibrary.VInterpTo` _returnvalue _returnvalue_2 DeltaSeconds 8.0))
    (if (< (`KismetMathLibrary.Vector_Distance` _returnvalue_2 _returnvalue) 1.0)
      (`self.SetShouldMove` false)
      (`self.HorseArrivedEvent`))
    (else
      (`self.K2_SetActorLocation` (`KismetMathLibrary.VInterpTo` (`self.K2_GetActorLocation`) (`self.TargetLocation`) DeltaSeconds 10.0)))))

(fn `SetTargetLocation`
  (params (NewParam :type "Vector Structure"))
  (set `self.TargetLocation` NewParam))

(fn `UserConstructionScript`)