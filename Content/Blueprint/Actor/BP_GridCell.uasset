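; BP_GridCell is a single board cell actor for the horse game, with an event to swap its mesh material.
; At BeginPlay it stores a target 300 units above its start, then eases up to it on Tick while ShouldMove is set.
; On arrival it stops and increments the ready counter in BP_HorseGameMode, calling AllReady when the count reaches 64.
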(event `self.SetMaterial`
  (params (MaterialInstance :type "Material Object Reference"))
  (`PrimitiveComponent.SetMaterial` (`self.GridCellMesh`) 0 MaterialInstance))

(event `self.ReceiveBeginPlay`
  (set `self.TargetLocation` (+ (`self.K2_GetActorLocation`) (0.0 0.0 300.0))))

(event `self.ReceiveTick`
  (params (DeltaSeconds :type "Float (single-precision)"))
  (if (`self.ShouldMove`)
    (`self.K2_SetActorLocation` (`KismetMathLibrary.VInterpTo` (`self.K2_GetActorLocation`) (`self.TargetLocation`) DeltaSeconds 6.0))
    (if (< (- (.z (`self.TargetLocation`)) (.z (`self.K2_GetActorLocation`))) 1.0)
      (set `self.ShouldMove` false)
      (bind _asbp_horse_game_mode (cast `/Game/Blueprint/BP_HorseGameMode` (`GameplayStatics.GetGameMode`)))
      (set `self.As BP Horse Game Mode` _asbp_horse_game_mode)
      (bind _output_get (set `HorseGameMode.ReadyGridCellNumber` (+ (`HorseGameMode.ReadyGridCellNumber` (`self.As BP Horse Game Mode`)) 1) (`self.As BP Horse Game Mode`)))
      (if (== _output_get 64)
        (`HorseGameMode.AllReady` (`self.As BP Horse Game Mode`))))))

(fn `UserConstructionScript`)